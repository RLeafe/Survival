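; Ammo pickup actor that refills the player's weapons when ThirdPersonCharacter_Female overlaps its trigger, then plays an explosion effect and pop sound and destroys itself.
; GiveAmmo runs once, finds world actors by the primary and secondary weapon classes, and sets their AmmoCapacity to AmmoTotal if either slot's class differs from BP_WeaponBase.
; On BeginPlay it spawns the same effect and animates the ammo with a rotation timeline that drives a bob timeline.
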(event `self.Trigger.OnComponentBeginOverlap`
  (params (OverlappedComponent :type "PrimitiveComponent Object Reference") (OtherActor :type "Actor Object Reference") (OtherComp :type "PrimitiveComponent Object Reference") (OtherBodyIndex :type Integer) (bFromSweep :type Boolean) (SweepResult :type "HitResult Structure (by ref)"))
  (bind _relativelocation (`SceneComponent.RelativeLocation` (`self.DefaultSceneRoot`)))
  ;[1 1 1] Check if player in trigger
  (cast `/Game/ODSMannequin/ThirdPersonBP/Blueprints/ThirdPersonCharacter_Female` OtherActor)
  (`self.GiveAmmo`)
  (`GameplayStatics.SpawnEmitterAtLocation` "/Game/CustomLevel/StarterContent/Particles/P_Explosion.P_Explosion" _relativelocation (struct) (0.5 0.5 0.5))
  (`GameplayStatics.PlaySoundAtLocation` "/Game/Audio/pop.pop" _relativelocation (struct) 0.25 1.0 0.0 null null null)
  (`self.K2_DestroyActor`))

(event `self.ReceiveBeginPlay`
  (bind _ammo (`self.Ammo`))
  (bind (_relativelocation_x _relativelocation_y) (`KismetMathLibrary.BreakVector` (`SceneComponent.RelativeLocation` _ammo)))
  ;[1 1 1] effects applied to ammo
  (`GameplayStatics.SpawnEmitterAtLocation` "/Game/CustomLevel/StarterContent/Particles/P_Explosion.P_Explosion" (`SceneComponent.RelativeLocation` (`self.DefaultSceneRoot`)) (struct) (0.5 0.5 0.5))
  (bind (_direction _rotation) (`Timeline|TL_Rotate`)
    (:`Update`
      (`SceneComponent.K2_SetRelativeRotation` _ammo (`KismetMathLibrary.MakeRotator` 0.0 0.0 _rotation) false false)
      (bind (_direction_2 _location) (`Timeline|TL_Bob`)
        (:`Update`
          (`SceneComponent.K2_SetRelativeLocation` _ammo (`KismetMathLibrary.MakeVector` _relativelocation_x _relativelocation_y _location) false false))))))

(event `GiveAmmo`
  (bind _asthird_person_character_female (cast `/Game/ODSMannequin/ThirdPersonBP/Blueprints/ThirdPersonCharacter_Female` (`GameplayStatics.GetPlayerCharacter` 0) :!pure true))
  (bind (_primaryweapon_class _primaryweapon_ammototal) (break `/Game/Blueprints/S_GunData` (`/Game/ODSMannequin/ThirdPersonBP/Blueprints/ThirdPersonCharacter_Female.primaryWeapon` _asthird_person_character_female)))
  (bind (_secondaryweapon_class _secondaryweapon_ammototal) (break `/Game/Blueprints/S_GunData` (`/Game/ODSMannequin/ThirdPersonBP/Blueprints/ThirdPersonCharacter_Female.secondaryWeapon` _asthird_person_character_female)))
  (bind _primaryweapon_class_2 (break `/Game/Blueprints/S_GunData` (`/Game/ODSMannequin/ThirdPersonBP/Blueprints/ThirdPersonCharacter_Female.primaryWeapon` _asthird_person_character_female)))
  (bind _secondaryweapon_class_2 (break `/Game/Blueprints/S_GunData` (`/Game/ODSMannequin/ThirdPersonBP/Blueprints/ThirdPersonCharacter_Female.secondaryWeapon` _asthird_person_character_female)))
  (`/Engine/EditorBlueprintResources/StandardMacros.DoOnce` false
    (:`Completed`
      (if (or (!= _primaryweapon_class_2 "/Game/Blueprints/BP_WeaponBase.BP_WeaponBase_C") (!= _secondaryweapon_class_2 "/Game/Blueprints/BP_WeaponBase.BP_WeaponBase_C"))
        (bind _returnvalue (`GameplayStatics.GetActorOfClass` _primaryweapon_class))
        (set `/Game/Blueprints/BP_WeaponBase.ammoCapacity` _primaryweapon_ammototal _returnvalue)
        (bind _returnvalue_2 (`GameplayStatics.GetActorOfClass` _secondaryweapon_class))
        (set `/Game/Blueprints/BP_WeaponBase.ammoCapacity` _secondaryweapon_ammototal _returnvalue_2)))))

(fn `UserConstructionScript`)