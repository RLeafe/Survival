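; BP_Target is a hittable target that flips to red when hit, then flips back to blue after a delay.
; TargetHit drives roll-rotation timelines through a DoOnce that resets after the flip back, with IsActive true only during the delay.
; BeginPlay stores the start location and, when UpDown or LeftRight is enabled, runs timelines that lerp the root along Z or X.
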(event `TargetHit`
  (bind _defaultsceneroot (`self.DefaultSceneRoot`))
  (bind (_returnvalue_roll _returnvalue_pitch _returnvalue_yaw) (`KismetMathLibrary.BreakRotator` (`SceneComponent.K2_GetComponentRotation` _defaultsceneroot)))
  (bind (_returnvalue_roll_2 _returnvalue_pitch_2 _returnvalue_yaw_2) (`KismetMathLibrary.BreakRotator` (`SceneComponent.K2_GetComponentRotation` _defaultsceneroot)))
  (if (not (`self.isHit`))
    (`/Engine/EditorBlueprintResources/StandardMacros.DoOnce` false :!label _label
      (:`Completed`
        ;[1 1 1] Flip to red
        (bind (_direction _fliptarget) (`Timeline|TL_isHitFlip` :!via `PlayFromStart`)
          (:`Update`
            (`SceneComponent.K2_SetWorldRotation` _defaultsceneroot (`KismetMathLibrary.MakeRotator` _fliptarget _returnvalue_pitch _returnvalue_yaw) false false))
          (:`Finished`
            ;[1 1 1] Allow delay so other targets can be hit
            (set `self.isActive` true)
            (`KismetSystemLibrary.Delay` (`self.resetDelay`))
            (set `self.isActive` false)
            ;[1 1 1] Reset to blue
            (bind (_direction_2 _resetflip) (`Timeline|TL_resetFlip` :!via `PlayFromStart`)
              (:`Update`
                (`SceneComponent.K2_SetWorldRotation` _defaultsceneroot (`KismetMathLibrary.MakeRotator` _resetflip _returnvalue_pitch_2 _returnvalue_yaw_2) false false))
              (:`Finished`
                (goto _label :!via `Reset`)))))))))

(event `self.ReceiveBeginPlay`
  (bind _defaultsceneroot (`self.DefaultSceneRoot`))
  (bind _defaultsceneroot_2 (`self.DefaultSceneRoot`))
  (bind (_returnvalue_x _returnvalue_y _returnvalue_z) (`KismetMathLibrary.BreakVector` (`SceneComponent.K2_GetComponentLocation` _defaultsceneroot_2)))
  (bind (_returnvalue_x_2 _returnvalue_y_2) (`KismetMathLibrary.BreakVector` (`SceneComponent.K2_GetComponentLocation` _defaultsceneroot)))
  (`|ExecutionSequence`
    (:`then_0`
      (`self.StartingLocation`))
    (:`then_1`
      ;[1 1 1] move up and down
      (if (`self.upDown`)
        (bind (_direction _alpha) (`Timeline|TL_UpDown` :!via `PlayFromStart`)
          (:`Update`
            (`SceneComponent.K2_SetWorldLocation` _defaultsceneroot (`KismetMathLibrary.VLerp` (`self.setStartLoc`) (`KismetMathLibrary.MakeVector` _returnvalue_x_2 _returnvalue_y_2 (`self.upLoc`)) _alpha) false false)))))
    (:`then_2`
      ;[1 1 1] move left and right
      (if (`self.leftRight`)
        (bind (_direction_2 _alpha_2) (`Timeline|TL_LeftRight`)
          (:`Update`
            (`SceneComponent.K2_SetWorldLocation` _defaultsceneroot_2 (`KismetMathLibrary.VLerp` (`self.setStartLoc`) (`KismetMathLibrary.MakeVector` (`self.leftLoc`) _returnvalue_y _returnvalue_z) _alpha_2) false false)))))))

(fn `UserConstructionScript`)