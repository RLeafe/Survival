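; Purchasable door that the player buys by holding Interact inside its trigger, with its price shown as text.
; Trigger overlap enables input and opens a gate, so a press starts the dissolve timeline if the female third-person character can afford it.
; The timeline drives the material's Appearance parameter; releasing early reverses it.
; A completed dissolve deducts money, plays a pop and explosion, and destroys the door.
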(event `self.ReceiveBeginPlay`
  (bind _output_get (set `self.costOfDoor` (`KismetTextLibrary.Conv_IntToText` (`self.doorPrice`))))
  (`TextRenderComponent.K2_SetText` (`self.PriceTxt`) _output_get))

(event `InputAction|Interact`
  (params (Key :type "Key Structure"))
  (bind _returnvalue (`SceneComponent.K2_GetComponentLocation` (`self.SM_Barrier_Prefab`)))
  (:`Pressed`
    ;[1 1 1] Is player in trigger and E is pressed
    (`/Engine/EditorBlueprintResources/StandardMacros.Gate` true :!label _label
      (:`Exit`
        (if (`self.hasBought`)
          _
          (elif (`self.CompareMoneyToPrice` (stale `self.Trigger.OnComponentBeginOverlap` _asthird_person_character_female))
            (`self.BuyDissolve`))))))
  (:`Released`
    ;[1 1 1] Buy Dissolve
    (if (not (`self.hasBought`))
      (`|ExecutionSequence`
        (:`then_0`
          (bind (_direction _alpha) (`Timeline|Timeline_0` :!via `Stop` :!label _label_2)
            (:`Update`
              (bind _returnvalue_2 (`KismetMathLibrary.Lerp` 0.0 1.0 _alpha))
              (`MeshComponent.SetScalarParameterValueOnMaterials` (`self.Unbought`) "Appearance" _returnvalue_2))
            (:`Finished`
              (if (<= _returnvalue_2 0.0)
                (`self.DecrementMoney` (stale `self.Trigger.OnComponentBeginOverlap` _asthird_person_character_female) (`self.doorPrice`))
                (set `self.hasBought` true)
                (`GameplayStatics.PlaySoundAtLocation` "/Game/Audio/pop.pop" _returnvalue (struct) 1.0 1.0 0.0 null null null)
                (`GameplayStatics.SpawnEmitterAtLocation` "/Game/CustomLevel/StarterContent/Particles/P_Explosion.P_Explosion" _returnvalue (struct) (5.0 5.0 5.0))
                (`self.K2_DestroyActor`)))))
        (:`then_1`
          (goto _label_2 :!via `Reverse`))))))

(event `self.Trigger.OnComponentBeginOverlap`
  (params (OverlappedComponent :type "PrimitiveComponent Object Reference") (OtherActor :type "Actor Object Reference") (OtherComp :type "PrimitiveComponent Object Reference") (OtherBodyIndex :type Integer) (bFromSweep :type Boolean) (SweepResult :type "HitResult Structure (by ref)"))
  ;[1 1 1] Is player in trigger and E is pressed
  (`self.EnableInput` (`GameplayStatics.GetPlayerController` 0))
  (bind _asthird_person_character_female (cast `/Game/ODSMannequin/ThirdPersonBP/Blueprints/ThirdPersonCharacter_Female` OtherActor))
  (goto _label :!via `Open`))

(event `self.Trigger.OnComponentEndOverlap`
  (params (OverlappedComponent :type "PrimitiveComponent Object Reference") (OtherActor :type "Actor Object Reference") (OtherComp :type "PrimitiveComponent Object Reference") (OtherBodyIndex :type Integer))
  ;[1 1 1] Is player in trigger and E is pressed
  (`self.DisableInput` (`GameplayStatics.GetPlayerController` 0))
  (cast `/Game/ODSMannequin/ThirdPersonBP/Blueprints/ThirdPersonCharacter_Female` OtherActor)
  (goto _label :!via `Close`))

(event `BuyDissolve`
  ;[1 1 1] Buy Dissolve
  (if (not (`self.hasBought`))
    (goto _label_2 :!via `PlayFromStart`)))

(fn `UserConstructionScript`)