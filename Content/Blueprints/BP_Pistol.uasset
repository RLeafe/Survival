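; Pistol weapon for the third-person player character, handling firing, reloading, ammo refills and saving its stats to the secondary slot on unequip.
; Fire spends a round, plays sound and montage, then line-traces from the follow camera with random spread, damaging zombies and triggering targets.
; Reload pools leftover rounds into the reserve and refills the magazine after a DoOnce-guarded delay.
; The construction script sets the stats; a muzzle trace sits unconnected.
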(event `self.Unequip`
  (set `/Game/ODSMannequin/ThirdPersonBP/Blueprints/ThirdPersonCharacter_Female.secondaryWeapon` (make `/Game/Blueprints/S_GunData` "BP_Pistol_C" (`self.totalRounds`) (`self.ammoCapacity`) (`self.ammoCount`) (`self.maxAmmo`) (`self.reloadTime`) (`self.bulletSpread`)) (`self.GetPlayerCast`)))

(event `self.Fire`
  (if (> (`self.ammoCount`) 0)
    (`self.AmmoCheck`)
    (`self.LineTrace`)
    (`|PlayMontage` (`Character.Mesh` (`self.GetPlayerCast`))) ; play the shooting animation montage
    (else
      (`GameplayStatics.PlaySoundAtLocation` "/Game/Audio/dryFire.dryFire" (`SceneComponent.K2_GetComponentLocation` (`/Game/ODSMannequin/ThirdPersonBP/Blueprints/ThirdPersonCharacter_Female.Gun` (`self.GetPlayerCast`))) (struct) 1.0 1.0 0.0 null null null))))

(event `self.Reload`
  (bind _asthird_person_character_female (`self.GetPlayerCast`))
  (bind _ammocapacity (`self.ammoCapacity`))
  (bind _maxammo (`self.maxAmmo`))
  (if (and (< (`self.ammoCount`) (`self.maxAmmo`)) (> (`self.ammoCapacity`) 0))
    (if (and (>= (`self.ammoCount`) 0) (> (`self.ammoCapacity`) 0))
      (set `self.remainingAmmo` (`self.ammoCount`))
      (set `self.ammoCapacity` (+ (`self.ammoCapacity`) (`self.remainingAmmo`)))
      (`/Engine/EditorBlueprintResources/StandardMacros.DoOnce` false :!label _label
        (:`Completed`
          (set `/Game/ODSMannequin/ThirdPersonBP/Blueprints/ThirdPersonCharacter_Female.isReloading` true _asthird_person_character_female)
          (`AnimInstance.Montage_Play` (`SkeletalMeshComponent.GetAnimInstance` (`Character.Mesh` _asthird_person_character_female)) null 1.0 "MontageLength" 0.0 true) ; Play reload animation
          (`KismetSystemLibrary.Delay` (`self.reloadTime`))
          (if (<= (`self.ammoCapacity`) (`self.maxAmmo`))
            (bind _output_get (set `self.ammoCount` _ammocapacity))
            (set `self.ammoCapacity` (- _output_get _output_get))
            (else
              (set `self.ammoCount` _maxammo)
              (set `self.ammoCapacity` (- _ammocapacity _maxammo))))
          (set `/Game/ODSMannequin/ThirdPersonBP/Blueprints/ThirdPersonCharacter_Female.isReloading` false _asthird_person_character_female)
          (goto _label :!via `Reset`))))))

(event `GiveAmmo`
  (set `self.ammoCapacity` (`self.totalRounds`))
  (`KismetSystemLibrary.PrintString` "Hello"))

(fn `AmmoCheck`
  (bind _returnvalue (`KismetMathLibrary.RandomFloatInRange` 1.0 1.9))
  (`/Engine/EditorBlueprintResources/StandardMacros.DecrementInt` (`self.ammoCount`)
    (:`  `
      (if (not (`/Game/ODSMannequin/ThirdPersonBP/Blueprints/ThirdPersonCharacter_Female.isReloading` (cast `/Game/ODSMannequin/ThirdPersonBP/Blueprints/ThirdPersonCharacter_Female` (`GameplayStatics.GetPlayerCharacter` 0) :!pure true)))
        (`GameplayStatics.PlaySoundAtLocation` "/Game/Audio/pop.pop" (`SceneComponent.K2_GetComponentLocation` (`/Game/ODSMannequin/ThirdPersonBP/Blueprints/ThirdPersonCharacter_Female.Gun` (`self.GetPlayerCast`))) (struct) (+ _returnvalue 1.3) _returnvalue 0.0 null null null)))))

(fn `LineTrace`
  (bind _bulletspread (`self.bulletSpread`))
  (bind _returnvalue (* _bulletspread -1.0))
  (bind _followcamera (`/Game/ODSMannequin/ThirdPersonBP/Blueprints/ThirdPersonCharacter_Female.FollowCamera` (cast `/Game/ODSMannequin/ThirdPersonBP/Blueprints/ThirdPersonCharacter_Female` (`GameplayStatics.GetPlayerCharacter` 0) :!pure true)))
  (bind _returnvalue_2 (`SceneComponent.K2_GetComponentLocation` _followcamera))
  (bind _outhit (`KismetSystemLibrary.LineTraceSingle` :`Start` _returnvalue_2 :`End` (+ (+ _returnvalue_2 (* (`SceneComponent.GetForwardVector` _followcamera) 20000.0)) (`KismetMathLibrary.MakeVector` (`KismetMathLibrary.RandomFloatInRange` _returnvalue) (`KismetMathLibrary.RandomFloatInRange` _returnvalue _bulletspread) (`KismetMathLibrary.RandomFloatInRange` _returnvalue _bulletspread))) :`TraceChannel` "TraceTypeQuery1" :`DrawDebugType` "ForDuration")) ; Camera Shot (Actual bullets)
  (`|ExecutionSequence`
    (:`then_0`
      (bind (_bblockinghit _binitialoverlap _time _distance _location _impactpoint _normal _impactnormal _physmat _hitactor) (`GameplayStatics.BreakHitResult` _outhit))
      (bind _aszombie_ai (cast `/Game/Characters/Zombie/Zombie_AI` _hitactor))
      (`GameplayStatics.ApplyDamage` _aszombie_ai (`self.damage`)))
    (:`then_1`
      (bind _asbp_target (cast `/Game/Blueprints/BP_Target` _hitactor))
      (`/Game/Blueprints/BP_Target.TargetHit` _asbp_target))))

(fn `UserConstructionScript`
  (`parent.UserConstructionScript`)
  (set `self.maxAmmo` 12)
  (set `self.ammoCount` 12)
  (set `self.reloadTime` 1.0)
  (set `self.bulletSpread` 25.0)
  (bind _output_get (set `self.ammoCapacity` 48))
  (set `self.totalRounds` _output_get))