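; BP_Gate is a gate that opens once every actor in its Targets array is active.
; Each Tick it loops over the targets and stops at the first inactive one.
; When all pass, a DoOnce plays the TL_OpenDoor timeline a single time, with no logic to close the gate again.
; The timeline curve sets the root's absolute world Z, keeping X and Y.
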(event `self.ReceiveTick`
  (params (DeltaSeconds :type "Float (single-precision)"))
  (bind _defaultsceneroot (`self.DefaultSceneRoot`))
  (bind (_returnvalue_x _returnvalue_y) (`KismetMathLibrary.BreakVector` (`SceneComponent.K2_GetComponentLocation` _defaultsceneroot)))
  (set `self.openDoor` true)
  ;[1 1 1] check if all active
  (for _array_element (`self.targets`)
    (if (not (`/Game/Blueprints/BP_Target.isActive` _array_element))
      (set `self.openDoor` false)
      (break)))
  (if (`self.openDoor`)
    (`/Engine/EditorBlueprintResources/StandardMacros.DoOnce` false
      (:`Completed`
        (bind (_direction _opendoor) (`Timeline|TL_OpenDoor` :!via `PlayFromStart`)
          (:`Update`
            (`SceneComponent.K2_SetWorldLocation` _defaultsceneroot (`KismetMathLibrary.MakeVector` _returnvalue_x _returnvalue_y _opendoor) false false)))))))

(fn `UserConstructionScript`)