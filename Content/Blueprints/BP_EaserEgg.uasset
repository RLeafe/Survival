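; BP_EaserEgg is an easter egg actor that triggers a one-time reward when every target in its Targets array is active.
; It polls each target's IsActive flag on Tick, stopping at the first inactive one.
; When all are active, a DoOnce sets the TextRender to the easter egg text and plays an explosion particle and sound at the root component's relative location.
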(event `self.ReceiveTick`
  (params (DeltaSeconds :type "Float (single-precision)"))
  (bind _relativelocation (`SceneComponent.RelativeLocation` (`self.DefaultSceneRoot`)))
  (set `self.targetsHit` true)
  ;[1 1 1] check if all active
  (for _array_element (`self.targets`)
    (if (not (`/Game/Blueprints/BP_Target.isActive` _array_element))
      (set `self.targetsHit` false)
      (break)))
  (if (`self.targetsHit`)
    (`/Engine/EditorBlueprintResources/StandardMacros.DoOnce` false
      (:`Completed`
        (`TextRenderComponent.K2_SetText` (`self.TextRender`) (`self.EasterEggTxt`))
        (`GameplayStatics.SpawnEmitterAtLocation` "/Game/CustomLevel/StarterContent/Particles/P_Explosion.P_Explosion" _relativelocation)
        (`GameplayStatics.PlaySoundAtLocation` "/Game/CustomLevel/StarterContent/Audio/Explosion_Cue.Explosion_Cue" _relativelocation (struct) 1.0 1.0 0.0 null null null)))))

(fn `UserConstructionScript`)