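; BP_Spawner is a wave-based zombie spawner that spawns a growing batch of Zombie_AI each wave.
; On BeginPlay it binds SpawnZombies to the NextWave event of ThirdPersonGameMode.
; Each spawn picks a random point in its Box, then a random navigable point near it.
; After each wave AddEnemy increments and is added to EnemiesSpawned, so wave size grows by an increasing step.
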(event `self.ReceiveBeginPlay`
  (bind _asthird_person_game_mode (cast `/Game/ODSMannequin/ThirdPersonBP/Blueprints/ThirdPersonGameMode` (`GameplayStatics.GetGameMode`)))
  (add `/Game/ODSMannequin/ThirdPersonBP/Blueprints/ThirdPersonGameMode.NextWave` _asthird_person_game_mode (delegate `SpawnZombies`)))

(event `SpawnZombies`
  (bind (_returnvalue_location _returnvalue_rotation) (`KismetMathLibrary.BreakTransform` (`self.GetTransform`)))
  ;[1 1 1] Spawn 1 extra per wave
  (for _ (range (`self.enemiesSpawned`))
    ;[1 1 1] Spawn at random point in box
    (`|SpawnActorFromClass` "/Game/Characters/Zombie/Zombie_AI.Zombie_AI_C" (`KismetMathLibrary.MakeTransform` (`NavigationSystemV1.K2_GetRandomLocationInNavigableRadius` (`KismetMathLibrary.RandomPointInBoundingBox` (`SceneComponent.K2_GetComponentLocation` (`self.DefaultSceneRoot`)) (`BoxComponent.GetScaledBoxExtent` (`self.Box`))) 100.0 null null) _returnvalue_rotation) "Undefined" "OverrideRootScale" null null))
  (`/Engine/EditorBlueprintResources/StandardMacros.IncrementInt` (`self.addEnemy`)
    (:`  `
      (set `self.enemiesSpawned` (+ (`self.enemiesSpawned`) (`self.addEnemy`))))))

(fn `UserConstructionScript`)